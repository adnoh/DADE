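; Playable pawn that moves and turns to follow touch input, with movement applied every tick until the touch ends.
; Swipe events store the touch point, and GetUnitVector derives a direction from its offset to the mesh's screen projection, multiplying deprojected position by direction.
; That vector drives movement input and yaw-only mesh rotation.
; Debug prints show touch and mesh coordinates plus the computed vector.
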(event TouchBegan(Swipe)
  (params (TouchLocation :type Vector%202D%20Structure) (Handle :type Integer))
  (bind _mesh (Variables|Character|GetMesh))
  ;[1 1 1] Touch Feed
  (Variables|Default|SetIsTouchEnd false)
  (Variables|Default|SetEnd TouchLocation)
  ;[1 1 1] Movement mk2
  (if (not (Variables|Default|GetIsTouchEnd))
    (bind _worldcoords (CallFunction|GetUnitVector (Game|GetPlayerController 0) (Transformation|GetWorldLocation _mesh) (Variables|Default|GetEnd)))
    (Pawn|Input|AddMovementInput _worldcoords 1.0 false)
    (CallFunction|GetRotateAnother _worldcoords _mesh)))

(event TouchMoved(Swipe)
  (params (TouchLocation :type Vector%202D%20Structure) (Handle :type Integer))
  (bind _mesh (Variables|Character|GetMesh))
  ;[1 1 1] Touch Feed
  (Variables|Default|SetIsTouchEnd false)
  (Variables|Default|SetEnd TouchLocation)
  ;[1 1 1] Movement mk2
  (if (not (Variables|Default|GetIsTouchEnd))
    (bind _worldcoords (CallFunction|GetUnitVector (Game|GetPlayerController 0) (Transformation|GetWorldLocation _mesh) (Variables|Default|GetEnd)))
    (Pawn|Input|AddMovementInput _worldcoords 1.0 false)
    (CallFunction|GetRotateAnother _worldcoords _mesh)))

(event TouchEnded(Swipe)
  (params (TouchLocation :type Vector%202D%20Structure) (Handle :type Integer))
  ;[1 1 1] Touch Feed
  (Variables|Default|SetIsTouchEnd true)
  (Variables|Default|SetEnd (.ScreenPosition (Class|GameplayStatics|ProjectWorldtoScreen (Game|GetPlayerController 0) (Transformation|GetWorldLocation (Variables|Character|GetMesh)) true))))

(event EventTick
  (params (DeltaSeconds :type Float%20%28single-precision%29))
  (bind _mesh (Variables|Character|GetMesh))
  ;[1 1 1] Tick
  (CallFunction|PrintCoords)
  ;[1 1 1] Movement mk2
  (if (not (Variables|Default|GetIsTouchEnd))
    (bind _worldcoords (CallFunction|GetUnitVector (Game|GetPlayerController 0) (Transformation|GetWorldLocation _mesh) (Variables|Default|GetEnd)))
    (Pawn|Input|AddMovementInput _worldcoords 1.0 false)
    (CallFunction|GetRotateAnother _worldcoords _mesh)))

(event EventBeginPlay
  (bind _returnvalue (Game|GetPlayerController 0))
  ;[1 1 1] BeginPlay
  (Variables|/Script/Engine.PlayerController|SetbShowMouseCursor _returnvalue true)
  (Variables|Default|SetEnd (.ScreenPosition (Class|GameplayStatics|ProjectWorldtoScreen _returnvalue (Transformation|GetWorldLocation (Variables|Character|GetMesh)) true))))

(fn ConstructionScript)

(fn GetUnitVector
  (params (Controller :type Player%20Controller%20Object%20Reference) (MeshCoords :type Vector) (ScrCoords :type Vector%202D%20Structure))
  (bind _screenposition (Class|GameplayStatics|ProjectWorldtoScreen Controller MeshCoords true))
  (bind (_x _y) (Math|Vector|BreakVector MeshCoords))
  (bind _returnvalue (- ScrCoords _screenposition))
  (bind _returnvalue_2 (Math|Vector2D|MakeVector2D _x _y))
  (bind _returnvalue_3 (Math|Vector2D|Normalize2D _returnvalue))
  (bind _returnvalue_4 (* _returnvalue_2 _returnvalue_3))
  (bind (_worldposition _worlddirection) (Class|GameplayStatics|DeprojectScreentoWorld Controller _returnvalue_4))
  (bind _returnvalue_5 (* _worldposition _worlddirection))
  (Development|PrintText (Utilities|Text|ToText(String) _returnvalue_5) true false "(R=1.000000,G=0.000000,B=0.066903,A=1.000000)" 0.001)
  (return _returnvalue_5))

(fn PrintCoords
  (bind _mesh (Variables|Character|GetMesh))
  (bind _returnvalue (Transformation|GetWorldLocation _mesh))
  (Development|PrintString (Utilities|String|Append "화면터치 // " (Utilities|String|ToString(Vector2d) (Variables|Default|GetEnd))) true true "(R=0.000000,G=0.660000,B=1.000000,A=1.000000)" 0.0001)
  (Development|PrintString (Utilities|String|Append "월드메쉬 // " (Utilities|String|ToString(Vector) _returnvalue)) true true "(R=0.000000,G=1.000000,B=0.119515,A=1.000000)" 0.0001)
  (Development|PrintString (Utilities|String|Append "화면메쉬 // " (Utilities|String|ToString(Vector2d) (.ScreenPosition (Class|GameplayStatics|ProjectWorldtoScreen (Game|GetPlayerController 0) _returnvalue true)))) true true "(R=0.000000,G=1.000000,B=0.119515,A=1.000000)" 0.0001)
  (Development|PrintString (Utilities|String|Append "메쉬벡터 // " (Utilities|String|ToString(Vector) _returnvalue)) true true "(R=1.000000,G=0.000000,B=0.820370,A=1.000000)" 0.001)
  (Development|PrintString (Utilities|String|Append "터치벡터 // " (Utilities|String|ToString(Vector) _returnvalue)) true true "(R=1.000000,G=0.000000,B=0.820370,A=1.000000)" 0.001))

(fn GetRotateAnother
  (params (TouchVector :type Vector) (Mesh :type Scene%20Component%20Object%20Reference))
  (bind _returnvalue (Transformation|GetWorldLocation Mesh))
  (Transformation|SetWorldRotation Mesh (Math|Rotator|MakeRotator 0.0 0.0 (.yaw (Math|Rotator|FindLookatRotation _returnvalue (+ _returnvalue TouchVector)))) true false)
  (return))